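; BP_Porte is a door that toggles open and closed each time a linked pressure plate fires its activation event.
; On BeginPlay it binds to the PlateIsActivate dispatcher of the referenced plate, if that reference is valid.
; A FlipFlop alternates the physics constraint's angular orientation target to swing the door on yaw, updating and printing the DoorIsOpen flag.
; An unused GetActorOfClass lookup remains as a rejected alternative.
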(event Custom|PlateIsActivateCall
  (Utilities|FlowControl|FlipFlop
    (:A
      (Variables|Default|SetbDoorIsOpen true)
      (Class|PhysicsConstraintComponent|SetAngularOrientationTarget (Variables|Default|GetPhysicsConstraint) (Math|Rotator|MakeRotator 0.0 0.0 -9e+01)))
    (:B
      (bind _output_get (Variables|Default|SetbDoorIsOpen false))
      (Class|PhysicsConstraintComponent|SetAngularOrientationTarget (Variables|Default|GetPhysicsConstraint) (Math|Rotator|MakeRotator 0.0 0.0 0.0))))
  (Development|PrintString (Utilities|String|Append "bDoorIsOpen :  " (Utilities|String|ToString(Boolean) _output_get))))

(event EventBeginPlay
  (bind _pressureplateref (Variables|Default|GetPressurePlateRef))
  (Utilities|IsValid _pressureplateref
    (:Is%20Valid
      (EventDispatchers|BindEventtoPlateIsActivate _pressureplateref (delegate Custom|PlateIsActivateCall)))))

(fn ConstructionScript)